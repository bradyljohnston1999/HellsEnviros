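; Interactable hinged door Blueprint that the player toggles open and closed with the Interact input.
; A Box overlap with bp_player shows a prompt widget and opens a gate that lets input through.
; After a short delay, the press also requires Islookingat, which it clears but nothing here sets.
; Separate timelines lerp door yaw for opening and closing, each with a sound, updating Isdoorclosed when finished.
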(event `self.ReceiveBeginPlay`
  (`self.EnableInput` (`GameplayStatics.GetPlayerController` 0)))

(event `InputAction|Interact` :consume false
  (params (Key :type "Key Structure"))
  (:`Pressed`
    (`KismetSystemLibrary.Delay` 0.2)
    (if (`self.islookingat?`)
      (set `self.islookingat?` false)
      (`/Engine/EditorBlueprintResources/StandardMacros.Gate` true :!label _label
        (:`Exit`
          (if (`self.isdoorclosed?`)
            (`GameplayStatics.PlaySound2D` "/Game/Zombie/Audio/Door/Open/do11.do11" 1.0 1.0 0.0 null null)
            (bind (_direction _open_close) (`Timeline|door open` :!via `PlayFromStart`)
              (:`Update`
                (`SceneComponent.K2_SetRelativeRotation` (`self.Door`) (`KismetMathLibrary.MakeRotator` 0.0 0.0 (`KismetMathLibrary.Lerp` (`self.CloseAngel`) (`self.Openangel`) _open_close)) false false))
              (:`Finished`
                (set `self.isdoorclosed?` false)))
            (else
              (`GameplayStatics.PlaySound2D` "/Game/Zombie/Audio/Door/Close/dc12_Cue.dc12_Cue" 1.0 1.0 0.0 null null)
              (bind (_direction_2 _open_close_2) (`Timeline|Timeline_0` :!via `ReverseFromEnd`)
                (:`Update`
                  (`SceneComponent.K2_SetRelativeRotation` (`self.Door`) (`KismetMathLibrary.MakeRotator` 0.0 0.0 (`KismetMathLibrary.Lerp` (`self.CloseAngel`) (`self.Openangel`) _open_close_2)) false false))
                (:`Finished`
                  (set `self.isdoorclosed?` true))))))))))

(event `self.Box.OnComponentBeginOverlap`
  (params (OverlappedComponent :type "PrimitiveComponent Object Reference") (OtherActor :type "Actor Object Reference") (OtherComp :type "PrimitiveComponent Object Reference") (OtherBodyIndex :type Integer) (bFromSweep :type Boolean) (SweepResult :type "HitResult Structure (by ref)"))
  (cast `/Game/Zombie/Blueprints/bp_player` OtherActor)
  (bind _returnvalue (`|CreateWidget` "/Game/Zombie/Blueprints/Interact_Prompt_Widget.Interact_Prompt_Widget_C"))
  (`UserWidget.AddToViewport` _returnvalue 0)
  (goto _label :!via `Open`))

(event `self.Box.OnComponentEndOverlap`
  (params (OverlappedComponent :type "PrimitiveComponent Object Reference") (OtherActor :type "Actor Object Reference") (OtherComp :type "PrimitiveComponent Object Reference") (OtherBodyIndex :type Integer))
  (cast `/Game/Zombie/Blueprints/bp_player` OtherActor)
  (`Widget.RemoveFromParent` (stale `self.Box.OnComponentBeginOverlap` _returnvalue))
  (goto _label :!via `Close`))

(fn `UserConstructionScript`)