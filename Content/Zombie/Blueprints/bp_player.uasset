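; First-person player character for a zombie game, handling movement, sprint, crouch, jump, mouse look, flashlight and a pause menu.
; Tick drives speed-based walk/run camera-shake headbob and aims the flashlight, while movement input runs a looping footstep timer.
; Interact both line-traces to flag a Door_bp and calls Interaction_interface on overlapping actors.
; PawnSensing freezes any bp_mannequin it sees, restoring walking through a short retriggerable delay once sightings stop.
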(event `self.K2_OnMovementModeChanged`
  (params (PrevMovementMode :type "EMovementMode Enum" :default "MOVE_None") (NewMovementMode :type "EMovementMode Enum" :default "MOVE_None") (PrevCustomMode :type Byte) (NewCustomMode :type Byte))
  (if (and (`|EnumEquality` PrevMovementMode "MOVE_Falling") (`|EnumEquality` NewMovementMode "MOVE_Walking"))
    (`self.Play Footstep Sound`)))

(event `Play Footstep Sound`
  (`GameplayStatics.PlaySoundAtLocation` "/Game/Zombie/Audio/Player_footsteps.Player_footsteps" (- (`self.K2_GetActorLocation`) (0.0 0.0 44.0)) (struct) 1.0 1.0 0.0 null null null))

(event `self.ReceiveTick`
  (params (DeltaSeconds :type "Float (single-precision)"))
  (`self.Headbob`)
  (`SceneComponent.K2_SetWorldRotation` (`self.SpotLight`) (`self.GetControlRotation`) false false))

(event `Headbob`
  (bind _returnvalue (`GameplayStatics.GetPlayerController` 0))
  (bind _returnvalue_2 (`KismetMathLibrary.VSize` (`self.GetVelocity`)))
  (if (and (> _returnvalue_2 0.0) (`self.CanJump`))
    (if (< _returnvalue_2 500.0)
      (`PlayerController.ClientStartCameraShakeFromSource` _returnvalue "/Game/Zombie/Blueprints/fpswalk.fpswalk_C" null)
      (else
        (`PlayerController.ClientStartCameraShakeFromSource` _returnvalue "/Game/Zombie/Blueprints/fpsrun.fpsrun_C" null)))))

(event `InputAction|sprint`
  (params (Key :type "Key Structure"))
  ;[1 1 1] basic movement
  (:`Pressed`
    (`self.Start Sprint`))
  (:`Released`
    (`self.Stop Sprint`)))

(event `InputAxis|Move Forward`
  (params (AxisValue :type "Float (single-precision)"))
  (bind (_returnvalue_x _returnvalue_y _returnvalue_z) (`KismetMathLibrary.BreakVector` (`self.GetVelocity`)))
  (bind (_returnvalue_roll _returnvalue_pitch _returnvalue_yaw) (`KismetMathLibrary.BreakRotator` (`self.GetControlRotation`)))
  ;[1 1 1] basic movement
  (`self.AddMovementInput` (`KismetMathLibrary.GetForwardVector` (`KismetMathLibrary.MakeRotator` 0.0 0.0 _returnvalue_yaw)) AxisValue)
  (if (and (or (> _returnvalue_x 2.0) (< _returnvalue_x -2.0) (> _returnvalue_y 2.0) (< 0.0 _returnvalue_y)) (== _returnvalue_z 0.0)) :!label _label
    (`/Engine/EditorBlueprintResources/StandardMacros.DoOnce` false :!label _label_2
      (:`Completed`
        (bind _returnvalue (`KismetSystemLibrary.K2_SetTimerDelegate` (delegate `Play Footstep Sound`) (`self.Footstep Inerval`) true))))
    (else
      (`KismetSystemLibrary.K2_ClearAndInvalidateTimerHandle` _returnvalue)
      (goto _label_2 :!via `Reset`))))

(event `InputAxis|Move Backwards`
  (params (AxisValue :type "Float (single-precision)"))
  (bind (_returnvalue_roll _returnvalue_pitch _returnvalue_yaw) (`KismetMathLibrary.BreakRotator` (`self.GetControlRotation`)))
  ;[1 1 1] basic movement
  (`self.AddMovementInput` (`KismetMathLibrary.GetForwardVector` (`KismetMathLibrary.MakeRotator` 0.0 0.0 _returnvalue_yaw)) AxisValue)
  (goto _label))

(event `InputAction|Jump`
  (params (Key :type "Key Structure"))
  ;[1 1 1] basic movement
  (:`Pressed`
    (`self.Jump`))
  (:`Released`
    (`self.StopJumping`)))

(event `InputAction|Crouch`
  (params (Key :type "Key Structure"))
  ;[1 1 1] basic movement
  (:`Pressed`
    (`self.Crouch`)
    (set `self.iscrouching?` true))
  (:`Released`
    (`self.UnCrouch`)
    (set `self.iscrouching?` false)))

(event `InputAxis|Move Left`
  (params (AxisValue :type "Float (single-precision)"))
  (bind (_returnvalue_roll _returnvalue_pitch _returnvalue_yaw) (`KismetMathLibrary.BreakRotator` (`self.GetControlRotation`)))
  ;[1 1 1] basic movement
  (`self.AddMovementInput` (`KismetMathLibrary.GetRightVector` (`KismetMathLibrary.MakeRotator` 0.0 0.0 _returnvalue_yaw)) AxisValue)
  (goto _label))

(event `InputAxis|Mouse Look Horizontal`
  (params (AxisValue :type "Float (single-precision)"))
  ;[1 1 1] basic movement
  (`self.AddControllerYawInput` (* AxisValue (`self.Mouse Sensitivity`) (`GameplayStatics.GetWorldDeltaSeconds`))))

(event `InputAxis|Move Right`
  (params (AxisValue :type "Float (single-precision)"))
  (bind (_returnvalue_roll _returnvalue_pitch _returnvalue_yaw) (`KismetMathLibrary.BreakRotator` (`self.GetControlRotation`)))
  ;[1 1 1] basic movement
  (`self.AddMovementInput` (`KismetMathLibrary.GetRightVector` (`KismetMathLibrary.MakeRotator` 0.0 0.0 _returnvalue_yaw)) AxisValue)
  (goto _label))

(event `InputAxis|Mouse Look Vertical`
  (params (AxisValue :type "Float (single-precision)"))
  ;[1 1 1] basic movement
  (`self.AddControllerPitchInput` (* AxisValue (`self.Mouse Sensitivity`) (`GameplayStatics.GetWorldDeltaSeconds`))))

(event `InputAction|Flashlight`
  (params (Key :type "Key Structure"))
  ;[1 1 1] Toggle On/Off Flashlight
  (:`Pressed`
    (`GameplayStatics.PlaySound2D` "/Game/Zombie/Audio/Click2-Sebastian-759472264.Click2-Sebastian-759472264" 1.0 1.0 0.0 null null)
    (if (`self.isflashlighton?`)
      (`self.TurnFlashlightOff`)
      (else
        (`self.TurnFlashlightON`)))))

(event `InputAction|Interact` :consume false
  (params (Key :type "Key Structure"))
  (bind _returnvalue (`self.K2_GetActorLocation`))
  (:`Pressed`
    (bind (_outhit _returnvalue_2) (`KismetSystemLibrary.LineTraceSingle` _returnvalue (+ _returnvalue (* (`SceneComponent.GetForwardVector` (`self.Camera`)) 400.0)) "TraceTypeQuery1"))
    (if _returnvalue_2
      (bind _asdoor_bp (cast `/Game/Zombie/Blueprints/Door_bp` (`.HitActor` (`GameplayStatics.BreakHitResult` _outhit))))
      (set `/Game/Zombie/Blueprints/Door_bp.islookingat?` true _asdoor_bp))))

(event `Key|X`
  (params (Key :type "Key Structure"))
  (:`Pressed`
    (`KismetSystemLibrary.PrintString` (`KismetStringLibrary.Conv_DoubleToString` (`self.Mouse Sensitivity`)))))

(event `InputAction|Pause` :paused true
  (params (Key :type "Key Structure"))
  (bind _returnvalue (`GameplayStatics.GetPlayerController` 0))
  ;[1 1 1] Pause
  (:`Pressed`
    (`/Engine/EditorBlueprintResources/StandardMacros.FlipFlop`
      (:`A`
        (bind _returnvalue_2 (`|CreateWidget` "/Game/Zombie/Pause_Menu/PauseMenuWidget.PauseMenuWidget_C"))
        (`UserWidget.AddToViewport` _returnvalue_2 0)
        (`GameplayStatics.SetGamePaused` true)
        (set `PlayerController.bShowMouseCursor` true _returnvalue))
      (:`B`
        (`Widget.RemoveFromParent` _returnvalue_2)
        (`GameplayStatics.SetGamePaused` false)
        (set `PlayerController.bShowMouseCursor` false _returnvalue)))))

(event `InputAction|Interact`
  (params (Key :type "Key Structure"))
  ;[1 1 1] control panel
  (:`Pressed`
    (for _array_element (`self.GetOverlappingActors` null)
      (bind _asinteraction_interface (cast `/Game/Zombie/Static_Camera/Interaction_interface` _array_element))
      (`/Game/Zombie/Static_Camera/Interaction_interface.ON Interaction` _asinteraction_interface self)
      (break))))

(event `self.PawnSensing.OnSeePawn`
  (params (Pawn :type "Pawn Object Reference"))
  (bind _asbp_mannequin (cast `/Game/Zombie/Blueprints/Mannequin/bp_mannequin` Pawn))
  (`|ExecutionSequence`
    (:`then_0`
      (bind _charactermovement (`Character.CharacterMovement` _asbp_mannequin))
      (`CharacterMovementComponent.DisableMovement` _charactermovement))
    (:`then_1`
      (`KismetSystemLibrary.RetriggerableDelay` 0.6)
      (`CharacterMovementComponent.SetMovementMode` _charactermovement "MOVE_Walking" 0))))

(fn `Start Sprint`
  (set `CharacterMovementComponent.MaxWalkSpeed` (`self.Sprint Speed`) (`self.CharacterMovement`)))

(fn `Stop Sprint`
  (set `CharacterMovementComponent.MaxWalkSpeed` (`self.Walk Speed`) (`self.CharacterMovement`)))

(fn `TurnFlashlightOff`
  (`SceneComponent.SetVisibility` (`self.SpotLight`) false false)
  (set `self.isflashlighton?` false))

(fn `TurnFlashlightON`
  (`SceneComponent.SetVisibility` (`self.SpotLight`) true false)
  (set `self.isflashlighton?` true))

(fn `UserConstructionScript`)