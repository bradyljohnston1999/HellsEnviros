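; Interactable control panel that lets one player at a time view a list of static cameras.
; On interaction, if it has cameras and is unoccupied, it stores the player, moves input from the pawn to the panel and switches the view to the first camera.
; Next and Previous inputs cycle the camera index with wraparound.
; Pressing Interact again returns view and input to the player and frees the panel.
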(event `/Game/Zombie/Static_Camera/Interaction_interface.ON Interaction`
  (params (Player :type "/Game/Zombie/Blueprints/bp_player Object Reference"))
  (bind _asplayer_controller (cast `PlayerController` (`Pawn.GetController` Player) :!pure true))
  (if (and (`self.Hascameras?`) (not (`self.Occupied?`)))
    (set `self.OccupiedPlayer` Player)
    (`self.DisableInput` Player _asplayer_controller)
    (`self.EnableInput` _asplayer_controller)
    (set `self.activecameraindex` 0)
    (`self.Set View Target as active camera`)))

(event `InputAction|Interact`
  (params (Key :type "Key Structure"))
  (bind _asplayer_controller (cast `PlayerController` (`Pawn.GetController` (`self.OccupiedPlayer`)) :!pure true))
  (:`Pressed`
    (`PlayerController.SetViewTargetWithBlend` _asplayer_controller (`self.OccupiedPlayer`) 0.0 "VTBlend_Linear" 0.0 false)
    (`self.EnableInput` (`self.OccupiedPlayer`) _asplayer_controller)
    (`self.DisableInput` _asplayer_controller)
    (set `self.OccupiedPlayer` null)))

(event `InputAction|Next  Camera`
  (params (Key :type "Key Structure"))
  (:`Pressed`
    (`self.increment camera index`)
    (`self.Set View Target as active camera`)))

(event `InputAction|Previous Camera`
  (params (Key :type "Key Structure"))
  (:`Pressed`
    (`self.decrement camera index`)
    (`self.Set View Target as active camera`)))

(fn `decrement camera index`
  (if (< (- (`self.activecameraindex`) 1) 0)
    (set `self.activecameraindex` (`KismetArrayLibrary.Array_LastIndex` (`self.static camera`)))
    (else
      (`/Engine/EditorBlueprintResources/StandardMacros.DecrementInt` (`self.activecameraindex`)))))

(fn `Hascameras?`
  (returns (ReturnValue :type Boolean))
  (return (> (`KismetArrayLibrary.Array_Length` (`self.static camera`)) 0)))

(fn `increment camera index`
  (if (> (+ (`self.activecameraindex`) 1) (`KismetArrayLibrary.Array_LastIndex` (`self.static camera`)))
    (set `self.activecameraindex` 0)
    (else
      (`/Engine/EditorBlueprintResources/StandardMacros.IncrementInt` (`self.activecameraindex`)))))

(fn `Occupied?`
  (returns (ReturnValue :type Boolean))
  (return (`KismetSystemLibrary.IsValid` (`self.OccupiedPlayer`))))

(fn `Set View Target as active camera`
  (`PlayerController.SetViewTargetWithBlend` (cast `PlayerController` (`Pawn.GetController` (`self.OccupiedPlayer`)) :!pure true) (`|GetArrayItem` (`self.static camera`) (`self.activecameraindex`)) 0.0 "VTBlend_Linear" 0.0 false))

(fn `UserConstructionScript`)